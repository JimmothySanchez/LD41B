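; Game mode for a foosball match that runs three timed rounds, tracks two team scores and returns to the main menu afterwards.
; Goal actors on the table report scores through bound events, which also top up the balls to the round's minimum.
; Tick drives the round clock; transitions clear balls, then arm barrier bumpers or play an expand sequence.
; The final round adds balls on a looping timer, while player 2 setup is empty.
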(event `self.ReceiveBeginPlay`
  (`|ExecutionSequence`
    (:`then_0`
      (bind _outactors (`GameplayStatics.GetAllActorsOfClass` "/Game/LD41Custom/Actors/BP_Table.BP_Table_C"))
      (set `self.TableReference` (`|GetArrayItem` _outactors)))
    (:`then_1`
      (`self.NextRound_EndTransition`))
    (:`then_2`
      ;[1 1 1] Add Score Hooks
      (bind _outactors_2 (`GameplayStatics.GetAllActorsOfClass` "/Game/LD41Custom/Actors/BP_Table.BP_Table_C"))
      (`|ExecutionSequence`
        (:`then_0`
          (bind _output (`|GetArrayItem` _outactors_2))
          (bind _asbp_goal (cast `/Game/LD41Custom/Actors/BP_goal` (`ChildActorComponent.ChildActor` (`/Game/LD41Custom/Actors/BP_Table.Team1Goal` _output))))
          (add `/Game/LD41Custom/Actors/BP_goal.Score` _asbp_goal (delegate `Score_Event_0`)))
        (:`then_1`
          (bind _asbp_goal_2 (cast `/Game/LD41Custom/Actors/BP_goal` (`ChildActorComponent.ChildActor` (`/Game/LD41Custom/Actors/BP_Table.Team2Goal` _output))))
          (add `/Game/LD41Custom/Actors/BP_goal.Score` _asbp_goal_2 (delegate `CustomEvent_0`)))))
    (:`then_3`
      (`self.SetUpPlayer2`))))

(event `self.ReceiveTick`
  (params (DeltaSeconds :type "Float (single-precision)"))
  (`self.UpdateGameTime` DeltaSeconds))

(event `Score_Event_0`
  ;[1 1 1] Add Score Hooks
  (`/Engine/EditorBlueprintResources/StandardMacros.IncrementInt` (`self.Team2Score`)
    (:`  `
      (`self.CheckBalls`))))

(event `CustomEvent_0`
  ;[1 1 1] Add Score Hooks
  (`/Engine/EditorBlueprintResources/StandardMacros.IncrementInt` (`self.Team1Score`)
    (:`  `
      (`self.CheckBalls`))))

(fn `ArmBarrierBumpers`
  (bind _outactors (`GameplayStatics.GetAllActorsOfClass` "/Game/LD41Custom/Actors/BP_Barrier.BP_Barrier_C"))
  (for _array_element _outactors
    (`/Game/LD41Custom/Actors/BP_Barrier.Arm` _array_element)))

(fn `CheckBalls`
  (locals (`lclMinimum Balls` :type Integer))
  (bind _outactors (`GameplayStatics.GetAllActorsOfClass` "/Game/LD41Custom/Actors/BP_Ball.BP_Ball_C"))
  (`|ExecutionSequence`
    (:`then_0`
      (switch `int` (`self.RoundNumber`)
        (:`Default`
          (set `local.lclMinimum Balls` 1 :!label _label))
        (:`0`
          (goto _label))
        (:`1`
          (goto _label))
        (:`2`
          (set `local.lclMinimum Balls` 3))
        (:`3`
          (goto _label))))
    (:`then_1`
      (if (< (`KismetArrayLibrary.Array_Length` _outactors) (`local.lclMinimum Balls`))
        (`/Game/LD41Custom/Actors/BP_Table.DropBall` (`self.TableReference`))))))

(fn `NextRound_EndTransition`
  (`|ExecutionSequence`
    (:`then_0`
      (set `self.RoundTime` 0.0)
      (set `self.TimerPaused` false)
      (`/Engine/EditorBlueprintResources/StandardMacros.IncrementInt` (`self.RoundNumber`)))
    (:`then_1`
      (switch `int` (`self.RoundNumber`)
        (:`1`
          (`/Game/LD41Custom/Actors/BP_Table.DropBall` (`self.TableReference`)))
        (:`2`
          (for _ (range 1 4)
            (`/Game/LD41Custom/Actors/BP_Table.DropBall` (`self.TableReference`))))
        (:`3`
          (`/Game/LD41Custom/Actors/BP_Table.DropBall` (`self.TableReference`))
          (bind _returnvalue (`KismetSystemLibrary.K2_SetTimer` self "Round3BallSpawn" 6.0 true))
          (set `self.BallSpawnTimer` _returnvalue))))))

(fn `NextRound_StartTransition`
  (`|ExecutionSequence`
    (:`then_0`
      ;[1 1 1] Remove Balls
      (bind _outactors (`GameplayStatics.GetAllActorsOfClass` "/Game/LD41Custom/Actors/BP_Ball.BP_Ball_C"))
      (for _array_element _outactors
        (`self.K2_DestroyActor` _array_element)))
    (:`then_1`
      (set `self.TimerPaused` true)
      (`KismetSystemLibrary.K2_PauseTimerHandle` (`self.BallSpawnTimer`)))
    (:`then_2`
      (switch `int` (`self.RoundNumber`)
        (:`0`
          (`KismetSystemLibrary.PrintString` "RoundNotWorking"))
        (:`1`
          (`self.ArmBarrierBumpers`)
          (`KismetSystemLibrary.K2_SetTimer` self "NextRound_EndTransition" 4.0))
        (:`2`
          (bind (_outactor _returnvalue) (`LevelSequencePlayer.CreateLevelSequencePlayer` "/Game/LD41Custom/Cinematics/LS_Expand.LS_Expand"))
          (add `MovieSceneSequencePlayer.OnStop` _returnvalue (`|CreateDelegate` :!event `NextRound_EndTransition`))
          (`MovieSceneSequencePlayer.Play` _returnvalue))
        (:`3`
          ;[1 1 1] Game End
          (set `self.GameOver` true)
          (`KismetSystemLibrary.K2_SetTimer` self "ReturnToMenu" 10.0))))))

(fn `ReturnToMenu`
  (bind _returnvalue (`GameplayStatics.GetPlayerController` 1))
  (`/Engine/EditorBlueprintResources/StandardMacros.IsValid` _returnvalue
    (:`Is Valid`
      (`GameplayStatics.RemovePlayer` _returnvalue))
    (:`Is Not Valid`
      _))
  (`GameplayStatics.OpenLevel` "MainMenu"))

(fn `Round3BallSpawn`
  (`/Game/LD41Custom/Actors/BP_Table.DropBall` (`self.TableReference`)))

(fn `SetUpPlayer2`)

(fn `UpdateGameTime`
  (params (TimeDelta :type "Float (double-precision)"))
  (if (not (`self.TimerPaused`))
    (set `self.RoundTime` (+ (`self.RoundTime`) TimeDelta))
    (if (>= (`self.RoundTime`) (`self.RoundMaxTime`))
      (`self.NextRound_StartTransition`))))

(fn `UserConstructionScript`)