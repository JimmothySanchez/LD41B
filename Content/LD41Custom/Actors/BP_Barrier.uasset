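; BP_Barrier is a team-owned barrier that holds three BP_Barrier_Bumper child actors behind a divider door.
; The construction script gives two bumpers the barrier's Team and the third the opposing team.
; Arm launches the door forward with physics and arms all bumpers.
; Tick then slides the Bumpers component sideways with a clamped, swept lerp over the arming duration, then destroys the door.
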(event `self.ReceiveTick`
  (params (DeltaSeconds :type "Float (single-precision)"))
  (if (`self.Arming`)
    (`|ExecutionSequence`
      (:`then_0`
        (set `self.ArmingDuration` (+ (`self.ArmingDuration`) DeltaSeconds)))
      (:`then_1`
        (`SceneComponent.K2_SetRelativeLocation` (`self.Bumpers`) (`KismetMathLibrary.VLerp` (0.0 0.0 0.0) (0.0 120.0 0.0) (`KismetMathLibrary.FClamp` (/ (`self.ArmingDuration`) (`self.ArmingDurationMax`)))) true false))
      (:`then_2`
        (if (>= (`self.ArmingDuration`) (`self.ArmingDurationMax`))
          (set `self.Arming` false)
          (`ActorComponent.K2_DestroyComponent` (`self.Barrier_DividerDoor`)))))))

(fn `Arm`
  (`PrimitiveComponent.SetSimulatePhysics` (`self.Barrier_DividerDoor`) true)
  (`PrimitiveComponent.SetPhysicsLinearVelocity` (`self.Barrier_DividerDoor`) (* (`self.GetActorForwardVector`) 1000.0) false "None")
  (`|ExecutionSequence`
    (:`then_0`
      (bind _asbp_barrier_bumper (cast `/Game/LD41Custom/Actors/BP_Barrier_Bumper` (`ChildActorComponent.ChildActor` (`self.ChildActor1`))))
      (set `/Game/LD41Custom/Actors/BP_Barrier_Bumper.Armed` true _asbp_barrier_bumper))
    (:`then_1`
      (bind _asbp_barrier_bumper_2 (cast `/Game/LD41Custom/Actors/BP_Barrier_Bumper` (`ChildActorComponent.ChildActor` (`self.ChildActor2`))))
      (set `/Game/LD41Custom/Actors/BP_Barrier_Bumper.Armed` true _asbp_barrier_bumper_2))
    (:`then_2`
      (bind _asbp_barrier_bumper_3 (cast `/Game/LD41Custom/Actors/BP_Barrier_Bumper` (`ChildActorComponent.ChildActor` (`self.ChildActor`))))
      (set `/Game/LD41Custom/Actors/BP_Barrier_Bumper.Armed` true _asbp_barrier_bumper_3))
    (:`then_3`
      (set `self.Arming` true)
      (set `self.ArmingDuration` 0.0))))

(fn `UserConstructionScript`
  (`|ExecutionSequence`
    (:`then_0`
      (bind _asbp_barrier_bumper (cast `/Game/LD41Custom/Actors/BP_Barrier_Bumper` (`ChildActorComponent.ChildActor` (`self.ChildActor2`))))
      (set `/Game/LD41Custom/Actors/BP_Barrier_Bumper.Team` (`self.Team`) _asbp_barrier_bumper))
    (:`then_1`
      (bind _asbp_barrier_bumper_2 (cast `/Game/LD41Custom/Actors/BP_Barrier_Bumper` (`ChildActorComponent.ChildActor` (`self.ChildActor`))))
      (switch `/Game/LD41Custom/Logic/Enum_Team` (`self.Team`)
        (:`NewEnumerator0`
          (set `/Game/LD41Custom/Actors/BP_Barrier_Bumper.Team` "NewEnumerator1" _asbp_barrier_bumper_2))
        (:`NewEnumerator1`
          (set `/Game/LD41Custom/Actors/BP_Barrier_Bumper.Team` "NewEnumerator0" _asbp_barrier_bumper_2))))
    (:`then_2`
      (bind _asbp_barrier_bumper_3 (cast `/Game/LD41Custom/Actors/BP_Barrier_Bumper` (`ChildActorComponent.ChildActor` (`self.ChildActor1`))))
      (set `/Game/LD41Custom/Actors/BP_Barrier_Bumper.Team` (`self.Team`) _asbp_barrier_bumper_3))))