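; BP_PlayerPaddles is a team-colored pair of left and right paddles that swing between down and up rotations.
; The construction script applies the team's material to both meshes.
; Each Tick, externally set LeftUp and RightUp flags drive clamped alphas at PaddleSpeed, which lerp each paddle's relative rotation.
; NeedLeftMovement is an unfinished stub, and neither it nor NeedRightMovement is called here.
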(event `self.ReceiveTick`
  (params (DeltaSeconds :type "Float (single-precision)"))
  (`self.UpdateLeftPaddle` DeltaSeconds)
  (`self.UpdateRightPaddle` DeltaSeconds))

(fn `NeedLeftMovement`
  (returns (MovementNeeded :type Boolean))
  (locals (CurrentRot :type "Float (double-precision)" :default 0.0))
  (set `local.CurrentRot` 0.0)
  (if (`self.LeftUp`)
    _))

(fn `NeedRightMovement`
  (returns (NeedMovement :type Boolean))
  (locals (lclRot :type "Float (double-precision)" :default 0.0))
  (set `local.lclRot` (.yaw (`SceneComponent.RelativeRotation` (`self.Right Paddle`))))
  (if (`self.RightUp`)
    (if (<= (`self.MaxRot`) (`local.lclRot`))
      (return true)
      (else
        (return false)))
    (elif (>= (`self.MinRot`) (`local.lclRot`))
      (return true)
      (else
        (return false)))))

(fn `UpdateLeftPaddle`
  (params (TimeDelta :type "Float (double-precision)"))
  (bind _returnvalue (* TimeDelta (`self.PaddleSpeed`)))
  (`|ExecutionSequence`
    (:`then_0`
      (if (`self.LeftUp`)
        (set `self.LerpLeftVal` (`KismetMathLibrary.FClamp` (+ (`self.LerpLeftVal`) _returnvalue)))
        (else
          (set `self.LerpLeftVal` (`KismetMathLibrary.FClamp` (- (`self.LerpLeftVal`) _returnvalue))))))
    (:`then_1`
      (`SceneComponent.K2_SetRelativeRotation` (`self.LeftPaddle`) (`KismetMathLibrary.RLerp` (`self.LeftDownRot`) (`self.LeftUpRot`) (`self.LerpLeftVal`) true) false false))))

(fn `UpdateRightPaddle`
  (params (TimeDelta :type "Float (double-precision)"))
  (bind _returnvalue (* TimeDelta (`self.PaddleSpeed`)))
  (`|ExecutionSequence`
    (:`then_0`
      (if (`self.RightUp`)
        (set `self.LerpRightVal` (`KismetMathLibrary.FClamp` (+ (`self.LerpRightVal`) _returnvalue)))
        (else
          (set `self.LerpRightVal` (`KismetMathLibrary.FClamp` (- (`self.LerpRightVal`) _returnvalue))))))
    (:`then_1`
      (`SceneComponent.K2_SetRelativeRotation` (`self.Right Paddle`) (`KismetMathLibrary.RLerp` (`self.RightDownRot`) (`self.RightUpRot`) (`self.LerpRightVal`) true) false false))))

(fn `UserConstructionScript`
  (switch `/Game/LD41Custom/Logic/Enum_Team` (`self.Team`)
    (:`NewEnumerator0`
      (`PrimitiveComponent.SetMaterial` (`self.LeftPaddle`) 1 "/Game/LD41Custom/Materials/Mat_Team1.Mat_Team1")
      (`PrimitiveComponent.SetMaterial` (`self.Right Paddle`) 1 "/Game/LD41Custom/Materials/Mat_Team1.Mat_Team1"))
    (:`NewEnumerator1`
      (`PrimitiveComponent.SetMaterial` (`self.LeftPaddle`) 1 "/Game/LD41Custom/Materials/Mat_Team2.Mat_Team2")
      (`PrimitiveComponent.SetMaterial` (`self.Right Paddle`) 1 "/Game/LD41Custom/Materials/Mat_Team2.Mat_Team2"))))