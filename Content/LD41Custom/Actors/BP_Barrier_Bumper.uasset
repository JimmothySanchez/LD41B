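; BP_Barrier_Bumper is a team-colored bumper barrier that knocks the ball away when armed.
; A BP_Ball entering its Box gets a force along the Arrow's forward vector and triggers a recoil.
; Recoil snaps the mesh to an offset, then Tick lerps it back to its relative origin over a set duration.
; The construction script picks the mesh's emissive material from Team.
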(event `self.ReceiveTick`
  (params (DeltaSeconds :type "Float (single-precision)"))
  (if (`self.Armed`)
    (`self.UpdateRecoil` DeltaSeconds)))

(event `self.Box.OnComponentBeginOverlap`
  (params (OverlappedComponent :type "PrimitiveComponent Object Reference") (OtherActor :type "Actor Object Reference") (OtherComp :type "PrimitiveComponent Object Reference") (OtherBodyIndex :type Integer) (bFromSweep :type Boolean) (SweepResult :type "HitResult Structure (by ref)"))
  (if (`self.Armed`)
    (if (== (`GameplayStatics.GetObjectClass` OtherActor) "/Game/LD41Custom/Actors/BP_Ball.BP_Ball_C")
      (bind _asbp_ball (cast `/Game/LD41Custom/Actors/BP_Ball` OtherActor))
      (`PrimitiveComponent.AddForce` (`/Game/LD41Custom/Actors/BP_Ball.Sphere` _asbp_ball) (* (`SceneComponent.GetForwardVector` (`self.Arrow`)) (`self.Force`)) "None" false)
      (`self.Recoil`))))

(fn `Recoil`
  (set `self.InRecoil` true)
  (set `self.RecoilDurration` 0.0)
  (`SceneComponent.K2_SetRelativeLocation` (`self.Barrier_DividerBumper`) (`self.RecoilPosition`) false false))

(fn `UpdateRecoil`
  (params (TimeDelta :type "Float (double-precision)"))
  (if (`self.InRecoil`)
    (`|ExecutionSequence`
      (:`then_0`
        (set `self.RecoilDurration` (+ (`self.RecoilDurration`) TimeDelta)))
      (:`then_1`
        (`SceneComponent.K2_SetRelativeLocation` (`self.Barrier_DividerBumper`) (`KismetMathLibrary.VLerp` (`self.RecoilPosition`) (0.0 0.0 0.0) (`KismetMathLibrary.FClamp` (/ (`self.RecoilDurration`) (`self.MaxRecoilDuration`)))) true false))
      (:`then_2`
        (if (>= (`self.RecoilDurration`) (`self.MaxRecoilDuration`))
          (set `self.InRecoil` false))))))

(fn `UserConstructionScript`
  (switch `/Game/LD41Custom/Logic/Enum_Team` (`self.Team`)
    (:`NewEnumerator0`
      (`PrimitiveComponent.SetMaterial` (`self.Barrier_DividerBumper`) 1 "/Game/LD41Custom/Materials/Mat_Team1_Emis.Mat_Team1_Emis"))
    (:`NewEnumerator1`
      (`PrimitiveComponent.SetMaterial` (`self.Barrier_DividerBumper`) 1 "/Game/LD41Custom/Materials/Mat_Team2_Emis.Mat_Team2_Emis"))))