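; BP_Barrier_Builder is a placement helper actor that builds a row of BP_Barrier actors.
; Its construction script loops Count times, adding child actor components spaced by Spacing along local X and centered on the actor.
; Each spawned barrier gets a Team value that alternates between two enum entries by odd or even index.
; The event graph holds only disabled stubs.
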(fn `UserConstructionScript`
  (for _index (range 1 (+ (`self.Count`) 1))
    (bind _returnvalue (`AddComponent|NODE_AddChildActorComponent-0` :`RelativeTransform` (`KismetMathLibrary.MakeTransform` (`KismetMathLibrary.MakeVector` (- (* (- _index 1) (`self.Spacing`)) (/ (* (- (`self.Count`) 1) (`self.Spacing`)) 2.0))))))
    (`ChildActorComponent.SetChildActorClass` _returnvalue "/Game/LD41Custom/Actors/BP_Barrier.BP_Barrier_C")
    (bind _asbp_barrier (cast `/Game/LD41Custom/Actors/BP_Barrier` (`ChildActorComponent.ChildActor` _returnvalue)))
    (if (== (mod _index 2) 1)
      (set `/Game/LD41Custom/Actors/BP_Barrier.Team` "NewEnumerator0" _asbp_barrier)
      (else
        (set `/Game/LD41Custom/Actors/BP_Barrier.Team` "NewEnumerator1" _asbp_barrier)))))