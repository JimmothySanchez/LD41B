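; BP_ManRow is an actor that builds a row of foosball men as static mesh components.
; Init stores the man count and spacing, then adds one FoosManMesh component per man along local X, centred on the actor origin.
; The construction script holds an unconnected copy of the same loop, so the row only appears when Init is called.
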(fn `Init`
  (params (InManCount :type Integer) (InManSpacing :type "Float (double-precision)"))
  (set `self.ManCount` InManCount)
  (set `self.ManSpacing` InManSpacing)
  (for _index (range (`self.ManCount`))
    (bind _returnvalue (`AddComponent|NODE_AddStaticMeshComponent-1` :`RelativeTransform` (`KismetMathLibrary.MakeTransform` (`KismetMathLibrary.MakeVector` (+ (* _index (`self.ManSpacing`)) (* (/ (* (- (`self.ManCount`) 1) (`self.ManSpacing`)) 2.0) -1.0))))))
    (`StaticMeshComponent.SetStaticMesh` _returnvalue (`self.FoosManMesh`))))

(fn `UserConstructionScript`)