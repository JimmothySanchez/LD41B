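; Player controller for a foosball game that lets each player work rows and paddles on the table and adds a HUD.
; BeginPlay finds BP_Table, caches this player's paddles and sends the initial row selection with a hardcoded player ID 0.
; Mouse and stick axes, scaled by separate multipliers, spin and strafe the active row by controller ID.
; Buttons pick or cycle three rows, bumpers set paddle up flags, and Exit quits.
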(event `self.ReceiveBeginPlay`
  (bind _returnvalue (`GameplayStatics.GetPlayerControllerID` self))
  (`KismetSystemLibrary.PrintString` (`KismetStringLibrary.Conv_IntToString` _returnvalue))
  (bind _outactors (`GameplayStatics.GetAllActorsOfClass` "/Game/LD41Custom/Actors/BP_Table.BP_Table_C"))
  (bind _output_get (set `self.TableRef` (`|GetArrayItem` _outactors)))
  (bind _returnvalue_2 (`GameplayStatics.GetPlayerControllerID` self))
  (bind _paddles (`/Game/LD41Custom/Actors/BP_Table.GetPlayerPadles` _output_get _returnvalue_2))
  (set `self.PaddleRef` _paddles)
  (bind _returnvalue_3 (`|CreateWidget` "/Game/LD41Custom/UI/Widget_HUD.Widget_HUD_C" self))
  (`UserWidget.AddToPlayerScreen` _returnvalue_3 0)
  (`/Game/LD41Custom/Actors/BP_Table.SetRowSelection` (`self.TableRef`) 0 (`self.ActiveRow`)))

(event `InputAxisKey|MouseX`
  (params (AxisValue :type "Float (single-precision)"))
  (bind _returnvalue (`GameplayStatics.GetPlayerControllerID` self))
  (`/Game/LD41Custom/Actors/BP_Table.UpdateRowRot` (`self.TableRef`) _returnvalue (`self.ActiveRow`) (* AxisValue (`self.SpinMultiplier`))))

(event `InputAxisKey|MouseY`
  (params (AxisValue :type "Float (single-precision)"))
  (bind _returnvalue (`GameplayStatics.GetPlayerControllerID` self))
  (`/Game/LD41Custom/Actors/BP_Table.UpdateRowStrafe` (`self.TableRef`) _returnvalue (`self.ActiveRow`) (* AxisValue (`self.LateralMovementMultiplier`))))

(event `InputAction|Row1`
  (params (Key :type "Key Structure"))
  (:`Pressed`
    (bind _output_get (set `self.ActiveRow` 0))
    (bind _returnvalue (`GameplayStatics.GetPlayerControllerID` self))
    (`/Game/LD41Custom/Actors/BP_Table.SetRowSelection` (`self.TableRef`) _returnvalue _output_get)))

(event `InputAxis|LateralMovement`
  (params (AxisValue :type "Float (single-precision)"))
  (bind _returnvalue (`GameplayStatics.GetPlayerControllerID` self))
  (`/Game/LD41Custom/Actors/BP_Table.UpdateRowStrafe` (`self.TableRef`) _returnvalue (`self.ActiveRow`) (* AxisValue (`self.StickMovementMultiplier`))))

(event `InputAction|Row2`
  (params (Key :type "Key Structure"))
  (:`Pressed`
    (bind _output_get (set `self.ActiveRow` 1))
    (bind _returnvalue (`GameplayStatics.GetPlayerControllerID` self))
    (`/Game/LD41Custom/Actors/BP_Table.SetRowSelection` (`self.TableRef`) _returnvalue _output_get)))

(event `InputAxis|Spin`
  (params (AxisValue :type "Float (single-precision)"))
  (bind _returnvalue (`GameplayStatics.GetPlayerControllerID` self))
  (`/Game/LD41Custom/Actors/BP_Table.UpdateRowRot` (`self.TableRef`) _returnvalue (`self.ActiveRow`) (* AxisValue (`self.StickSpinMultiplier`))))

(event `InputAction|Row3`
  (params (Key :type "Key Structure"))
  (:`Pressed`
    (bind _output_get (set `self.ActiveRow` 2))
    (bind _returnvalue (`GameplayStatics.GetPlayerControllerID` self))
    (`/Game/LD41Custom/Actors/BP_Table.SetRowSelection` (`self.TableRef`) _returnvalue _output_get)))

(event `InputAction|Exit`
  (params (Key :type "Key Structure"))
  (:`Pressed`
    (`KismetSystemLibrary.QuitGame` null "Quit")))

(event `InputAction|LeftBumper`
  (params (Key :type "Key Structure"))
  (:`Pressed`
    (set `/Game/LD41Custom/Actors/BP_PlayerPaddles.LeftUp` true (`self.PaddleRef`)))
  (:`Released`
    (set `/Game/LD41Custom/Actors/BP_PlayerPaddles.LeftUp` false (`self.PaddleRef`))))

(event `InputAction|RightBumper`
  (params (Key :type "Key Structure"))
  (:`Pressed`
    (set `/Game/LD41Custom/Actors/BP_PlayerPaddles.RightUp` true (`self.PaddleRef`)))
  (:`Released`
    (set `/Game/LD41Custom/Actors/BP_PlayerPaddles.RightUp` false (`self.PaddleRef`))))

(event `InputAction|PreviousRow`
  (params (Key :type "Key Structure"))
  (:`Pressed`
    (set `self.ActiveRow` (+ (`self.ActiveRow`) -1))
    (if (< (`self.ActiveRow`) 0)
      (set `self.ActiveRow` 2))
    (bind _returnvalue (`GameplayStatics.GetPlayerControllerID` self))
    (`/Game/LD41Custom/Actors/BP_Table.SetRowSelection` (`self.TableRef`) _returnvalue (`self.ActiveRow`))))

(event `InputAction|NextRow`
  (params (Key :type "Key Structure"))
  (:`Pressed`
    (bind _output_get (set `self.ActiveRow` (mod (+ (`self.ActiveRow`) 1) 3)))
    (bind _returnvalue (`GameplayStatics.GetPlayerControllerID` self))
    (`/Game/LD41Custom/Actors/BP_Table.SetRowSelection` (`self.TableRef`) _returnvalue _output_get)))

(fn `UserConstructionScript`)