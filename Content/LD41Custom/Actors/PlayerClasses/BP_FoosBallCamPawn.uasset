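; Camera pawn for a foosball game that turns its camera to follow the balls in play.
; Each Tick, UpdateCameras finds all BP_Ball actors and, with one or two present, smoothly rotates toward a point from GetActorMidpoints, otherwise easing back to zero relative rotation.
; For two balls that point is half their position difference, not the true midpoint, as the corrective offset is left unused.
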(event `self.ReceiveBeginPlay`)

(event `self.ReceiveTick`
  (params (DeltaSeconds :type "Float (single-precision)"))
  (`self.UpdateCameras` DeltaSeconds))

(fn `GetActorMidpoints`
  (params (Actors :type "Array of Actor Object Reference"))
  (returns (Center :type "Vector Structure"))
  (locals (CenterLocation :type "Vector Structure" :default (0.0 0.0 0.0)))
  (for (_array_element _array_index) Actors
    (if (== _array_index 0)
      (bind _returnvalue (`self.K2_GetActorLocation` _array_element))
      (set `local.CenterLocation` _returnvalue)
      (else
        (set `local.CenterLocation` (- (`local.CenterLocation`) _returnvalue)))))
  (return (/ (`local.CenterLocation`) (`KismetMathLibrary.Conv_IntToDouble` (`KismetArrayLibrary.Array_Length` Actors)))))

(fn `UpdateCameras`
  (params (TimeDelta :type "Float (double-precision)"))
  (locals (lclTimeDelta :type "Float (double-precision)"))
  (set `local.lclTimeDelta` TimeDelta)
  (bind _outactors (`GameplayStatics.GetAllActorsOfClass` "/Game/LD41Custom/Actors/BP_Ball.BP_Ball_C"))
  (bind _returnvalue (`KismetArrayLibrary.Array_Length` _outactors))
  (if (and (> _returnvalue 0) (<= _returnvalue 2))
    (bind _center (`self.GetActorMidpoints` _outactors))
    (`SceneComponent.K2_SetWorldRotation` (`self.Camera`) (`KismetMathLibrary.RInterpTo` (`SceneComponent.K2_GetComponentRotation` (`self.Camera`)) (`KismetMathLibrary.FindLookAtRotation` (`SceneComponent.K2_GetComponentLocation` (`self.Camera`)) _center) (`local.lclTimeDelta`) 3.0) false false)
    (else
      (`SceneComponent.K2_SetRelativeRotation` (`self.Camera`) (`KismetMathLibrary.RInterpTo` (`SceneComponent.RelativeRotation` (`self.Camera`)) (struct) (`local.lclTimeDelta`) 3.0) false false))))

(fn `UserConstructionScript`)