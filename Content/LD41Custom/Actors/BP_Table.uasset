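; Foosball-style table actor for two teams, with three child-actor man rows and a paddles actor per team.
; The construction script interleaves the rows along Y by RowSpacing, then sets each one's team, man count and spacing.
; Functions look up rows by player and index to slide them within the row's LateralMax or spin them on roll.
; DropBall spawns a BP_Ball at the spawn point with a random-direction velocity.
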(fn `DropBall`
  (bind _returnvalue (`|SpawnActorFromClass` "/Game/LD41Custom/Actors/BP_Ball.BP_Ball_C" (`SceneComponent.K2_GetComponentToWorld` (`self.BallSpawnPoint`)) "Undefined" "OverrideRootScale" null null))
  (`PrimitiveComponent.SetPhysicsLinearVelocity` (`/Game/LD41Custom/Actors/BP_Ball.Sphere` _returnvalue) (* (`KismetMathLibrary.RandomUnitVector`) 1000.0) false "None"))

(fn `GetPlayerPadles`
  (params (PlayerId :type Integer))
  (returns (paddles :type "/Game/LD41Custom/Actors/BP_PlayerPaddles Object Reference"))
  (switch `int` PlayerId
    (:`0`
      (bind _asbp_player_paddles (cast `/Game/LD41Custom/Actors/BP_PlayerPaddles` (`ChildActorComponent.ChildActor` (`self.Team1Paddles`))))
      (return _asbp_player_paddles))
    (:`1`
      (bind _asbp_player_paddles_2 (cast `/Game/LD41Custom/Actors/BP_PlayerPaddles` (`ChildActorComponent.ChildActor` (`self.Team2Paddles`))))
      (return _asbp_player_paddles_2))))

(fn `GetRowActor`
  (params (Player :type Integer) (Row :type Integer))
  (returns (SelectedRow :type "/Game/LD41Custom/Actors/BP_ManRow Object Reference"))
  (locals (lclRow :type "/Game/LD41Custom/Actors/BP_ManRow Object Reference"))
  (`|ExecutionSequence`
    (:`then_0`
      (switch `int` Player
        (:`0`
          (switch `int` Row
            (:`0`
              (bind _asbp_man_row (cast `/Game/LD41Custom/Actors/BP_ManRow` (`ChildActorComponent.ChildActor` (`self.Team1_Row1`))))
              (set `local.lclRow` _asbp_man_row))
            (:`1`
              (bind _asbp_man_row_2 (cast `/Game/LD41Custom/Actors/BP_ManRow` (`ChildActorComponent.ChildActor` (`self.Team1_Row2`))))
              (set `local.lclRow` _asbp_man_row_2))
            (:`2`
              (bind _asbp_man_row_3 (cast `/Game/LD41Custom/Actors/BP_ManRow` (`ChildActorComponent.ChildActor` (`self.Team1_Row3`))))
              (set `local.lclRow` _asbp_man_row_3))))
        (:`1`
          (switch `int` Row
            (:`0`
              (bind _asbp_man_row_4 (cast `/Game/LD41Custom/Actors/BP_ManRow` (`ChildActorComponent.ChildActor` (`self.Team2_Row1`))))
              (set `local.lclRow` _asbp_man_row_4))
            (:`1`
              (bind _asbp_man_row_5 (cast `/Game/LD41Custom/Actors/BP_ManRow` (`ChildActorComponent.ChildActor` (`self.Team2_Row2`))))
              (set `local.lclRow` _asbp_man_row_5))
            (:`2`
              (bind _asbp_man_row_6 (cast `/Game/LD41Custom/Actors/BP_ManRow` (`ChildActorComponent.ChildActor` (`self.Team2_Row3`))))
              (set `local.lclRow` _asbp_man_row_6))))))
    (:`then_1`
      (return (`local.lclRow`)))))

(fn `GetRowComponent`
  (params (Player :type Integer) (Row :type Integer))
  (returns (SelectedRow :type "ChildActorComponent Object Reference"))
  (locals (rtrnRow :type "ChildActorComponent Object Reference"))
  (`|ExecutionSequence`
    (:`then_0`
      (switch `int` Player
        (:`0`
          (switch `int` Row
            (:`0`
              (set `local.rtrnRow` (`self.Team1_Row1`)))
            (:`1`
              (set `local.rtrnRow` (`self.Team1_Row2`)))
            (:`2`
              (set `local.rtrnRow` (`self.Team1_Row3`)))))
        (:`1`
          (switch `int` Row
            (:`0`
              (set `local.rtrnRow` (`self.Team2_Row1`)))
            (:`1`
              (set `local.rtrnRow` (`self.Team2_Row2`)))
            (:`2`
              (set `local.rtrnRow` (`self.Team2_Row3`)))))))
    (:`then_1`
      (return (`local.rtrnRow`)))))

(fn `UpdateRowRot`
  (params (PlayerId :type Integer) (RowNumber :type Integer) (Value :type "Float (double-precision)"))
  (bind _selectedrow (`self.GetRowComponent` PlayerId RowNumber))
  (`SceneComponent.K2_AddRelativeRotation` _selectedrow (`KismetMathLibrary.MakeRotator` Value) false false))

(fn `UpdateRowStrafe`
  (params (Player :type Integer) (RowNumber :type Integer) (Value :type "Float (double-precision)"))
  (locals (lclRow :type "ChildActorComponent Object Reference"))
  (bind _selectedrow (`self.GetRowComponent` Player RowNumber))
  (bind _output_get (set `local.lclRow` _selectedrow))
  (bind _selectedrow_2 (`self.GetRowActor` Player RowNumber))
  (bind _lateralmax (`/Game/LD41Custom/Actors/BP_ManRow.LateralMax` _selectedrow_2))
  (`SceneComponent.K2_SetRelativeLocation` _output_get (`KismetMathLibrary.MakeVector` (`KismetMathLibrary.FClamp` (+ Value (.x (`SceneComponent.RelativeLocation` (`local.lclRow`)))) (* _lateralmax -1.0) _lateralmax) (.y (`SceneComponent.RelativeLocation` (`local.lclRow`))) (.z (`SceneComponent.RelativeLocation` (`local.lclRow`)))) true false))

(fn `UserConstructionScript`
  (`|ExecutionSequence`
    (:`then_0`
      ;[1 1 1] Team1 Row 2
      (`SceneComponent.K2_SetRelativeTransform` (`self.Team1_Row2`) (`KismetMathLibrary.MakeTransform` (`KismetMathLibrary.MakeVector` 0.0 (* (`self.RowSpacing`) -0.5))) false false)
      (bind _asbp_man_row (cast `/Game/LD41Custom/Actors/BP_ManRow` (`ChildActorComponent.ChildActor` (`self.Team1_Row2`))))
      (set `/Game/LD41Custom/Actors/BP_ManRow.Team` "NewEnumerator0" _asbp_man_row)
      (`/Game/LD41Custom/Actors/BP_ManRow.Init` _asbp_man_row 5 (`self.ManSpacing`)))
    (:`then_1`
      ;[1 1 1] Team1 Row 1
      (`SceneComponent.K2_SetRelativeTransform` (`self.Team1_Row1`) (`KismetMathLibrary.MakeTransform` (`KismetMathLibrary.MakeVector` 0.0 (* (`self.RowSpacing`) -2.5))) false false)
      (bind _asbp_man_row_2 (cast `/Game/LD41Custom/Actors/BP_ManRow` (`ChildActorComponent.ChildActor` (`self.Team1_Row1`))))
      (set `/Game/LD41Custom/Actors/BP_ManRow.Team` "NewEnumerator0" _asbp_man_row_2)
      (`/Game/LD41Custom/Actors/BP_ManRow.Init` _asbp_man_row_2 2 (`self.ManSpacing`)))
    (:`then_2`
      ;[1 1 1] Team1 Row 3
      (`SceneComponent.K2_SetRelativeTransform` (`self.Team1_Row3`) (`KismetMathLibrary.MakeTransform` (`KismetMathLibrary.MakeVector` 0.0 (* (`self.RowSpacing`) 1.5))) false false)
      (bind _asbp_man_row_3 (cast `/Game/LD41Custom/Actors/BP_ManRow` (`ChildActorComponent.ChildActor` (`self.Team1_Row3`))))
      (set `/Game/LD41Custom/Actors/BP_ManRow.Team` "NewEnumerator0" _asbp_man_row_3)
      (`/Game/LD41Custom/Actors/BP_ManRow.Init` _asbp_man_row_3 3 (`self.ManSpacing`)))
    (:`then_3`
      ;[1 1 1] Team2 Row 2
      (`SceneComponent.K2_SetRelativeTransform` (`self.Team2_Row2`) (`KismetMathLibrary.MakeTransform` (`KismetMathLibrary.MakeVector` 0.0 (* (`self.RowSpacing`) 0.5))) false false)
      (bind _asbp_man_row_4 (cast `/Game/LD41Custom/Actors/BP_ManRow` (`ChildActorComponent.ChildActor` (`self.Team2_Row2`))))
      (set `/Game/LD41Custom/Actors/BP_ManRow.Team` "NewEnumerator1" _asbp_man_row_4)
      (`/Game/LD41Custom/Actors/BP_ManRow.Init` _asbp_man_row_4 5 (`self.ManSpacing`)))
    (:`then_4`
      ;[1 1 1] Team2 Row 1
      (`SceneComponent.K2_SetRelativeTransform` (`self.Team2_Row1`) (`KismetMathLibrary.MakeTransform` (`KismetMathLibrary.MakeVector` 0.0 (* (`self.RowSpacing`) 2.5))) false false)
      (bind _asbp_man_row_5 (cast `/Game/LD41Custom/Actors/BP_ManRow` (`ChildActorComponent.ChildActor` (`self.Team2_Row1`))))
      (set `/Game/LD41Custom/Actors/BP_ManRow.Team` "NewEnumerator1" _asbp_man_row_5)
      (`/Game/LD41Custom/Actors/BP_ManRow.Init` _asbp_man_row_5 2 (`self.ManSpacing`)))
    (:`then_5`
      ;[1 1 1] Team2 Row 3
      (`SceneComponent.K2_SetRelativeTransform` (`self.Team2_Row3`) (`KismetMathLibrary.MakeTransform` (`KismetMathLibrary.MakeVector` 0.0 (* (`self.RowSpacing`) -1.5))) false false)
      (bind _asbp_man_row_6 (cast `/Game/LD41Custom/Actors/BP_ManRow` (`ChildActorComponent.ChildActor` (`self.Team2_Row3`))))
      (set `/Game/LD41Custom/Actors/BP_ManRow.Team` "NewEnumerator1" _asbp_man_row_6)
      (`/Game/LD41Custom/Actors/BP_ManRow.Init` _asbp_man_row_6 3 (`self.ManSpacing`)))))